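; BP_Door is an interactable door that swings open or closed each time its Interact event fires.
; Interact flips IsOpen and either plays the DoorOpenClose timeline from the start to open or reverses it to close.
; The timeline drives the Door component's relative yaw through a half turn, so reopening mid-close restarts from fully closed.
; IsInteracting always returns false, and no tick logic is used.
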(event EventBeginPlay)

(event Collision|EventActorBeginOverlap
  (params (OtherActor :type Actor%20Object%20Reference)))

(event EventTick
  (params (DeltaSeconds :type Float%20%28single-precision%29)))

(event EventInteract
  (params (InteractingPlayer :type Character%20Object%20Reference))
  (bind _door (Variables|Default|GetDoor))
  (bind _relativerotation (Variables|/Script/Engine.SceneComponent|GetRelativeRotation _door))
  ;[0.15 0.15 0.15 0.5] Door Interaction: Opens and closes door
  (if (Variables|Default|GetIsOpen)
    (Variables|Default|SetIsOpen false)
    (bind _dooranimtrack (Timeline|DoorOpenClose Reverse)
      (:Update
        (Transformation|SetRelativeRotation _door (Math|Rotator|MakeRotator (.roll _relativerotation) (.pitch _relativerotation) (Math|Float|Lerp 0.0 1.8e+02 _dooranimtrack)) false false)))
    (else
      (Variables|Default|SetIsOpen true)
      (Timeline|DoorOpenClose PlayFromStart))))

(fn ConstructionScript)

(fn IsInteracting
  (params (InteractingPlayer :type Character%20Object%20Reference))
  (return false))