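; Customer NPC character that claims a spline path from NPC_Manager_BP and can sit on seats it overlaps.
; On BeginPlay it takes the manager's path at the current capacity index, then increments that count; an exposed function returns the path.
; Tick sets walk speed from the manager's customer speed, or zero when unable to move.
; Seat overlap with CanSit set loops a sitting animation, switches to flying mode and snaps to the seat's position and facing.
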(event OnComponentBeginOverlap(CapsuleComponent)
  (params (OverlappedComponent :type Primitive%20Component%20Object%20Reference) (OtherActor :type Actor%20Object%20Reference) (OtherComp :type Primitive%20Component%20Object%20Reference) (OtherBodyIndex :type Integer) (bFromSweep :type Boolean) (SweepResult :type Hit%20Result%20Structure%20%28by%20ref%29))
  ;[0.009756 0.5938 0.198 0.5] Collision check with seat bp
  (bind _asseat_bp (Utilities|Casting|CastToSeat_BP OtherActor))
  (bind _output_get (Variables|Default|SetSeat _asseat_bp))
  (Utilities|IsValid _output_get
    (:Is%20Valid
      (if (Variables|Default|GetCan%20Sit?)
        (bind _output_get_2 (Variables|Default|SetIs%20Sitting? true))
        (CallFunction|SitinSeatLocation _output_get_2)
        (else
          (Variables|Default|SetIs%20Sitting? false))))))

(event Custom|Assign%20NPC%20Entrance%20Path
  ;[0.009756 0.5938 0.198 0.5] Assign NPC Entrance Path
  (bind _returnvalue (Actor|GetActorOfClass "/Game/NPCSystem/NPC_Management/NPC_Manager_BP.NPC_Manager_BP_C"))
  (bind _output_get (Variables|Default|SetNPC%20Manager _returnvalue))
  (Utilities|IsValid _output_get
    (:Is%20Valid
      (bind _output_get_2 (Variables|Default|SetSpline%20Path%20BP (Utilities|Array|Get(acopy) (Variables|/Game/NPCSystem/NPC_Management/NPC_Manager_BP.NPC_Manager_BP_C|GetSpline%20NPC%20Path%20Array _output_get) (Variables|/Game/NPCSystem/NPC_Management/NPC_Manager_BP.NPC_Manager_BP_C|GetCapacity _output_get))))
      (Development|PrintText (Utilities|Text|FormatText "{NPC Name} has been assigned: {spline Path}" self _output_get_2) true true "(R=1.000000,G=0.232195,B=0.000000,A=1.000000)" 5.0))))

(event Custom|Sit%20In%20Seat%20Location
  (params (Is%20Sitting? :type Boolean))
  (bind _seat (Variables|Default|GetSeat))
  (bind _billboard (Variables|/Game/NPCSystem/Seats/Seat_BP.Seat_BP_C|GetBillboard _seat))
  (bind _returnvalue (Transformation|GetWorldLocation _billboard))
  ;[0.009756 0.5938 0.198 0.5] Sit in seat location
  (if Is%20Sitting?
    (Variables|Default|SetCan%20Move? false)
    (Components|Animation|PlayAnimation (Variables|Character|GetMesh) "/Game/Mixamo/Sitting_UE.Sitting_UE" true)
    (Pawn|Components|CharacterMovement|SetMovementMode (Variables|Character|GetCharacterMovement) "MOVE_Flying" 0)
    (Transformation|SetActorRotation (Transformation|GetWorldRotation (Variables|/Game/NPCSystem/Seats/Seat_BP.Seat_BP_C|GetFront%20Arrow _seat)))
    (Transformation|SetActorLocation (Math|Vector|MakeVector (.x _returnvalue) (.y _returnvalue) (+ (.z _returnvalue) 43.0)) false false)))

(event EventBeginPlay
  ;[0.009756 0.5938 0.198 0.5] Assign NPC Path and increase capacity count
  (CallFunction|AssignNPCEntrancePath :!pinned true) ; Assign spline path when customer spawns
  (Math|Integer|IncrementInt (Variables|/Game/NPCSystem/NPC_Management/NPC_Manager_BP.NPC_Manager_BP_C|GetCapacity (Variables|Default|GetNPC%20Manager)) :!pinned true) ; Add +1 to capacity count
)

(event Collision|EventActorBeginOverlap
  (params (OtherActor :type Actor%20Object%20Reference)))

(event EventTick
  (params (DeltaSeconds :type Float%20%28single-precision%29))
  (bind _charactermovement (Variables|Character|GetCharacterMovement))
  ;[0.009756 0.5938 0.198 0.5] Instance movement speed control
  (if (Variables|Default|GetCan%20Move?)
    (Variables|/Script/Engine.CharacterMovementComponent|SetMaxWalkSpeed _charactermovement (Variables|/Game/NPCSystem/NPC_Management/NPC_Manager_BP.NPC_Manager_BP_C|GetCustomer%20Speed (Variables|Default|GetNPC%20Manager)))
    (else
      (Variables|/Script/Engine.CharacterMovementComponent|SetMaxWalkSpeed _charactermovement 0.0))))

(fn ConstructionScript)

(fn NPCSplineMovement
  (return (Variables|Default|GetSpline%20Path%20BP)))