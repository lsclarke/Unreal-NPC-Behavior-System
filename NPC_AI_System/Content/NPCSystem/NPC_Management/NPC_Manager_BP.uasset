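; NPC manager Blueprint that drives customer spawning and table service in a restaurant.
; Every tick it runs two capacity check macros and, if SpawnSwitch is on, has the CustomerSpawner create a customer after a delay.
; It then rebuilds the customer array from all Customer_BP actors and links a customer to a spline path indexed by Capacity.
; Tick also starts service on the current table section, advancing the index when that entry is invalid.
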(event Custom|Spawn%20Customers
  ;[0.009756 0.5938 0.198 0.5] Spawn Customers
  (if (Variables|Default|GetSpawn%20Switch?)
    (Utilities|FlowControl|Delay (Variables|Default|GetSpawn%20Delay))
    (Default|SpawnNewCostumer (Variables|Default|GetCustomer%20Spawner) "/Game/NPCSystem/Customer_NPC/Customer_BP.Customer_BP_C")
    (bind _outactors (Actor|GetAllActorsOfClass "/Game/NPCSystem/Customer_NPC/Customer_BP.Customer_BP_C"))
    (bind _output_get (Variables|Default|SetCustomer%20NPC%20Array _outactors))
    (Variables|/Game/NPCSystem/NPC_Management/NPC_Spline_Path_BP.NPC_Spline_Path_BP_C|SetNPC%20Customer (Utilities|Array|Get(acopy) (Variables|Default|GetSpline%20NPC%20Path%20Array) (- (Variables|Default|GetCapacity) 1)) (Utilities|Array|Get(acopy) _output_get (Variables|Default|GetCapacity)))))

(event Custom|Check%20Capacity
  ;[0.009756 0.5938 0.198 0.5] Check Capacity
  (if (Utilities|If((Capacity<0)OR(Capacity!=MaxCapacity)))
    (if (Utilities|If(CustomerNPCArrayLength<MaxCapacity))
      (CallFunction|SpawnCustomers)
      (else
        (Development|PrintString "Fail Fire 2")))))

(event EventBeginPlay)

(event Collision|EventActorBeginOverlap
  (params (OtherActor :type Actor%20Object%20Reference)))

(event EventTick
  (params (DeltaSeconds :type Float%20%28single-precision%29))
  (bind _table_sections_array (Variables|Default|GetTable%20Sections%20Array))
  (bind _table_index (Variables|Default|GetTable%20Index))
  (bind _output (Utilities|Array|Get(acopy) _table_sections_array _table_index))
  ;[0.009756 0.5938 0.198 0.5] Event Tick
  (CallFunction|CheckCapacity)
  (Utilities|IsValid _output
    (:Is%20Valid
      (Default|StartService _output))
    (:Is%20Not%20Valid
      (Math|Integer|IncrementInt (Variables|Default|GetTable%20Index)))))

(fn ConstructionScript)