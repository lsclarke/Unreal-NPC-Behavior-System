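; NPC spline path Blueprint that supplies waypoint locations along a spline for a customer NPC.
; IncrementPath advances the PathPoint index, clamping against the spline's length rather than its point count.
; FindSplineLocation returns the world location at that index on the SplinePath of a supplied path Blueprint.
; AssignCustomerToSpline stores the first entry of the NPC manager's customer array when the manager is valid.
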(event Custom|Increment%20Path
  (bind _spline_path (Variables|Default|GetSpline%20Path))
  (bind _returnvalue (Spline|GetSplineLength _spline_path))
  ;[0.009756 0.5938 0.198 0.5] Increase path point
  (if (> (Variables|Default|GetPath%20Point) _returnvalue)
    (Variables|Default|SetPath%20Point (Math|Float|Truncate _returnvalue))
    (else
      (Variables|Default|SetPath%20Point (+ (Variables|Default|GetPath%20Point) 1)))))

(event Custom|Assign%20Customer%20To%20Spline
  ;[0.009756 0.5938 0.198 0.5] Assign customer to spline
  (Utilities|IsValid (Variables|Default|GetNPC%20Manager)
    (:Is%20Valid
      (Variables|Default|SetNPC%20Customer (Utilities|Array|Get(acopy) (Variables|/Game/NPCSystem/NPC_Management/NPC_Manager_BP.NPC_Manager_BP_C|GetCustomer%20NPC%20Array (Variables|Default|GetNPC%20Manager)))))))

(event EventBeginPlay)

(event Collision|EventActorBeginOverlap
  (params (OtherActor :type Actor%20Object%20Reference)))

(event EventTick
  (params (DeltaSeconds :type Float%20%28single-precision%29)))

(fn ConstructionScript)

(fn FindSplineLocation
  (params (Spline%20Path%20BP :type NPC%20Spline%20Path%20BP%20Object%20Reference))
  ;[0.009756 0.5938 0.198 0.5] Finds location of spline point in spline path
  (return (Spline|GetLocationatSplinePoint (Variables|NPC_Spline_Path_BP_C|GetSpline%20Path Spline%20Path%20BP) (Variables|Default|GetPath%20Point) "World")))