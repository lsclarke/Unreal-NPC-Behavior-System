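; Waiter NPC character that services restaurant tables and pauses to take orders.
; Finds the NPC manager on BeginPlay and sets walk speed every Tick from MovementSpeed and a CanMove flag.
; SetWaiterOrderService refills OrderOfService with every table in the level when an occupied table is missing from it.
; TakeOrder halts movement for a short delay, and NPCSplineMovement exposes the waiter's spline path.
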(event Custom|Set%20Waiter%20Order%20Service
  (bind _table_array (Variables|Default|GetTable%20Array))
  ;[0.009756 0.5938 0.198 0.5] Set waiter order service
  (for _array_element _table_array
    (Utilities|IsValid _array_element
      (:Is%20Valid
        (if (> (Variables|/Game/NPCSystem/Table_Section_BPs/Table_BP.Table_BP_C|GetSeats%20Filled%20Count _array_element) 0)
          (if (!= (Utilities|Array|ContainsItem _table_array _array_element) (Utilities|Array|ContainsItem (Variables|Default|GetOrder%20Of%20Service) _array_element))
            (bind _outactors (Actor|GetAllActorsOfClass "/Game/NPCSystem/Table_Section_BPs/Table_BP.Table_BP_C"))
            (Variables|Default|SetOrder%20Of%20Service _outactors)))))))

(event Custom|Take%20Order
  (Development|PrintString "Taking order")
  (Variables|Default|Setmovement%20speed 0.0)
  (Utilities|FlowControl|Delay 3.0)
  (Variables|Default|Setmovement%20speed 3e+02))

(event EventBeginPlay
  (bind _returnvalue (Actor|GetActorOfClass "/Game/NPCSystem/NPC_Management/NPC_Manager_BP.NPC_Manager_BP_C"))
  (Utilities|IsValid _returnvalue
    (:Is%20Valid
      (Variables|Default|SetNPC%20Manager _returnvalue))))

(event Collision|EventActorBeginOverlap
  (params (OtherActor :type Actor%20Object%20Reference)))

(event EventTick
  (params (DeltaSeconds :type Float%20%28single-precision%29))
  (bind _charactermovement (Variables|Character|GetCharacterMovement))
  ;[0.009756 0.5938 0.198 0.5] Instance movement speed control
  (if (Variables|Default|GetCan%20Move?)
    (Variables|/Script/Engine.CharacterMovementComponent|SetMaxWalkSpeed _charactermovement (Variables|Default|Getmovement%20speed))
    (else
      (Variables|/Script/Engine.CharacterMovementComponent|SetMaxWalkSpeed _charactermovement 0.0))))

(fn ConstructionScript)

(fn NPCSplineMovement
  (return (Variables|Default|GetSpline%20Path%20BP)))